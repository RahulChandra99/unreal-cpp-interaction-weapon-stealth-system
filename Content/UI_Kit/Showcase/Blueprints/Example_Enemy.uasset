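; Showcase enemy character for the UI kit that demonstrates a world-space health bar and minimap marker.
; On BeginPlay it sets up the bar and registers with Minimap widgets; Tick turns the bar toward the camera.
; Damage updates the bar; death triggers ragdoll, timed removal and a follow-up ShowcaseText.
; FireBullet faces the player and launches a Bullet using a suggested projectile velocity; the construction script tints the mannequin materials.
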(event EventBeginPlay
  (bind _asgradient_bar_base (Utilities|Casting|CastToGradientBar_Base (UserInterface|GetUserWidgetObject (Variables|Default|GetHealth%20Bar))))
  (Variables|/Game/UI_Kit/Widgets/GradientBars/GradientBar_Base.GradientBar_Base_C|SetBarID _asgradient_bar_base "health")
  (Variables|/Game/UI_Kit/Widgets/GradientBars/GradientBar_Base.GradientBar_Base_C|SetColor _asgradient_bar_base "(R=0.390000,G=0.000000,B=0.000000,A=1.000000)")
  (EventDispatchers|BindEventtoUpdateHealthBar (EventDispatchers|CreateEvent _asgradient_bar_base :!event UpdateBar))
  (Default|CallUpdateHealthBar "health" (/ (Variables|Default|GetCurrent%20Health) (Variables|Default|GetMaximum%20Health)))
  (bind _foundwidgets (Widget|GetAllWidgetsOfClass "/Game/UI_Kit/Widgets/Misc/Minimap_Base.Minimap_Base_C" false))
  (for _array_element _foundwidgets
    (bind _asminimap_base (Utilities|Casting|CastToMinimap_Base _array_element))
    (Default|AddPointOfInterest _asminimap_base self "(R=0.630000,G=0.074329,B=0.000000,A=1.000000)")))

(event EventTick
  (params (DeltaSeconds :type Float%20%28single-precision%29))
  (Utilities|IsValid (Variables|Default|GetHealth%20Bar)
    (:Is%20Valid
      (Transformation|SetWorldRotation (Variables|Default|GetHealth%20Bar) (Math|Rotator|FindLookatRotation (Transformation|GetWorldLocation (Variables|Default|GetHealth%20Bar)) (Transformation|GetActorLocation (Game|GetPlayerCameraManager 0))) false false))))

(event Game|Damage|EventAnyDamage
  (params (Damage :type Float%20%28single-precision%29) (DamageType :type Damage%20Type%20Object%20Reference) (InstigatedBy :type Controller%20Object%20Reference) (DamageCauser :type Actor%20Object%20Reference))
  (bind _output_get (Variables|Default|SetCurrent%20Health (- (Variables|Default|GetCurrent%20Health) Damage)))
  (Default|CallUpdateHealthBar "health" (/ _output_get (Variables|Default|GetMaximum%20Health)))
  (if (<= (Variables|Default|GetCurrent%20Health) 0.0)
    (Utilities|FlowControl|DoOnce false
      (:Completed
        (Class|SkeletalMeshComponent|SetAllBodiesSimulatePhysics (Variables|Character|GetMesh) true)
        (Collision|SetCollisionEnabled (Variables|Collision|GetCapsuleComponent) "NoCollision")
        (Components|DestroyComponent (Variables|Default|GetHealth%20Bar))
        (Class|Pawn|DetachfromControllerPendingDestroy)
        (Actor|SetLifeSpan 1e+01)
        (Utilities|FlowControl|Delay 1.0)
        (Game|SpawnActorfromClass "/Game/UI_Kit/Showcase/Blueprints/ShowcaseText.ShowcaseText_C" (Math|Conversions|ToTransform(Vector) (Transformation|GetActorLocation)) "AlwaysSpawn" 0 "There are several types of objectives and 
you can easily add your own! 
Move forward now to see a few other layouts!" 0)))))

(fn ConstructionScript
  (bind _returnvalue (Rendering|Material|CreateDynamicMaterialInstance "/Game/UI_Kit/Mannequin/Character/Materials/M_UE4Man_Body.M_UE4Man_Body" :!class /Script/Engine.KismetMaterialLibrary))
  (Rendering|Material|SetVectorParameterValue _returnvalue "BodyColor" "(R=0.030000,G=0.030000,B=0.030000,A=1.000000)" :!class /Script/Engine.MaterialInstanceDynamic)
  (Rendering|Material|SetMaterial (Variables|Character|GetMesh) 0 _returnvalue)
  (bind _returnvalue_2 (Rendering|Material|CreateDynamicMaterialInstance "/Game/UI_Kit/Mannequin/Character/Materials/M_UE4Man_ChestLogo.M_UE4Man_ChestLogo" :!class /Script/Engine.KismetMaterialLibrary))
  (Rendering|Material|SetVectorParameterValue _returnvalue_2 "BodyColor" "(R=0.090000,G=0.000000,B=0.000000,A=1.000000)" :!class /Script/Engine.MaterialInstanceDynamic)
  (Rendering|Material|SetMaterial (Variables|Character|GetMesh) 1 _returnvalue_2))

(fn FireBullet
  (Transformation|SetActorRotation (Math|Rotator|FindLookatRotation (Transformation|GetActorLocation) (Transformation|GetActorLocation (Game|GetPlayerCharacter 0))))
  (bind (_tossvelocity _returnvalue) (Class|GameplayStatics|BlueprintSuggestProjectileVelocity (Transformation|GetWorldLocation (Variables|Default|GetProjectile%20Spawn)) (Transformation|GetActorLocation (Game|GetPlayerCharacter 0)) 3e+03 0.0 "OnlyTraceWhileAsceding" 3e+01 false false))
  (if _returnvalue
    (Game|SpawnActorfromClass "/Game/UI_Kit/Showcase/Blueprints/Bullet.Bullet_C" (Math|Conversions|ToTransform(Vector) (Transformation|GetWorldLocation (Variables|Default|GetProjectile%20Spawn))) "Undefined" 0 _tossvelocity 0)))