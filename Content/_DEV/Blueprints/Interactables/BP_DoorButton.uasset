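; BP_DoorButton is an interactable button that opens and closes a linked door, with a "Press Button" prompt.
; Interact plays a click sound, then plays or reverses a timeline based on IsDoorOpened.
; The timeline slides RespectiveDoor's mesh along relative X at a fixed Z, despite its track being named ZRotation.
; On finish it toggles IsDoorOpened and clears IsInteracting.
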(event EventInteract
  (params (InterActor :type Actor%20Object%20Reference))
  (Audio|PlaySoundatLocation "/Engine/VREditor/Sounds/UI/Click_on_Button.Click_on_Button" (Transformation|GetActorLocation) "0, 0, 0" 1.0 1.0 0.0 0 0 0 0)
  (if (not (Variables|Default|GetbIsDoorOpened))
    (bind _zrotation (Timeline|Timeline Play)
      (:Update
        (Transformation|SetRelativeLocation (Variables|/Game/_DEV/Blueprints/Interactables/BP_InteractItemBase.BP_InteractItemBase_C|GetMesh (Variables|Default|GetRespectiveDoor)) (Math|Vector|MakeVector _zrotation 0.0 -1e+02) false false))
      (:Finished
        (if (Variables|Default|GetbIsDoorOpened)
          (Variables|Default|SetbIsDoorOpened false)
          (else
            (Variables|Default|SetbIsDoorOpened true)))
        (Variables|Default|SetbIsInteracting false)))
    (else
      (Timeline|Timeline Reverse))))

(fn ConstructionScript
  (|CallParentFunction))

(fn GetItemRef
  (return self))

(fn GetTypeOfInteraction
  (return "NewEnumerator0"))

(fn GetInteractionText
  (return (Utilities|Text|FormatText "Press Button") "/Game/_DEV/Misc/KeyboardButtons/keyboard_e.keyboard_e"))