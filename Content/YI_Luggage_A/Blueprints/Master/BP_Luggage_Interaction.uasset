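; Interactive luggage prop that players can open and close, or optionally knock into physics simulation on contact.
; Editor events randomize scale, pose, yaw and material on an instanced static mesh, for one unlocked actor or all of them.
; At runtime it destroys that instance, using a dynamic static mesh for open/closed swaps with sound and particles, or a simulated skeletal mesh on player overlap.
; Skeletal hits play velocity-scaled, throttled impact sounds.
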(event OnComponentBeginOverlap(Box)
  (params (OverlappedComponent :type Primitive%20Component%20Object%20Reference) (OtherActor :type Actor%20Object%20Reference) (OtherComp :type Primitive%20Component%20Object%20Reference) (OtherBodyIndex :type Integer) (bFromSweep :type Boolean) (SweepResult :type Hit%20Result%20Structure%20%28by%20ref%29))
  ;[1 1 1] Edit this to reference your characters blueprint
  (Utilities|Casting|CastToBP_FirstPersonCharacter OtherActor)
  (CallFunction|SetDynamic))

(event OnComponentHit(SkeletalMesh)
  (params (HitComponent :type Primitive%20Component%20Object%20Reference) (OtherActor :type Actor%20Object%20Reference) (OtherComp :type Primitive%20Component%20Object%20Reference) (NormalImpulse :type Vector :default "0, 0, 0") (Hit :type Hit%20Result%20Structure%20%28by%20ref%29))
  (bind _soundphysics (Variables|Default|GetSoundPhysics))
  ;[0.1194 1 0 1 36] Physics Collision Sound Effects
  (if (Variables|Default|GetSoundReady)
    (bind _returnvalue (Physics|GetPhysicsLinearVelocity (Variables|Default|GetSkeletalMesh) "None"))
    (Utilities|FlowControl|Sequence
      (:then_0
        (Utilities|FlowControl|DoOnce false
          (:Completed
            (Audio|SpawnSoundatLocation _soundphysics "0, 0, 0" "0, 0, 0" (Math|Float|MapRangeClamped (Math|Vector|VectorLength _returnvalue) 1e+03 1e+01 0.1 1.0) 1.0 0.0 0 0))))
      (:then_1
        (Utilities|FlowControl|Delay (Math|Random|RandomFloatinRange 0.1 0.2))
        (if (> (Math|Vector|VectorLength _returnvalue) 2e+01)
          (Audio|SpawnSoundatLocation _soundphysics (.Location (Collision|BreakHitResult Hit)) "0, 0, 0" (Math|Float|MapRangeClamped (Math|Vector|VectorLength _returnvalue) 1e+03 1e+01 0.1 1.0) 1.0 0.0 0 0)
          (Variables|Default|SetSoundReady false)
          (Utilities|FlowControl|Delay 0.35)
          (Variables|Default|SetSoundReady true))))))

(event Custom|Randomize%20All
  ;[1 1 1] Editor Buttons and Generation
  (bind _outactors (Actor|GetAllActorsOfClass "BP_Luggage_Interaction_C"))
  (for _array_element _outactors
    (CallFunction|Generate _array_element)))

(event Custom|Generate
  ;[1 1 1] Editor Buttons and Generation
  (if (not (Variables|Default|GetLocked))
    (|RandomizationParameters)))

(event Custom|PlayerInteraction
  (CallFunction|OpenLuggage))

(event Custom|SetDynamic
  (bind _skeletalmesh (Variables|Default|GetSkeletalMesh))
  (Utilities|FlowControl|DoOnce false
    (:Completed
      (Utilities|DestroyInstance)
      (if (Variables|Default|GetPhysicsSimulationOnImpact?)
        (Variables|Default|SetDynamicSkeletalSpawned true)
        (Components|DestroyComponent (Variables|Default|GetDynamicMesh))
        (Transformation|SetRelativeTransform (Variables|Default|GetSkeletalMesh) (Variables|Default|GetTransform_Original) false false)
        (Rendering|Material|SetMaterial _skeletalmesh 0 (Variables|Default|GetAssignMaterial))
        (Components|SkinnedMesh|SetSkinnedAssetandUpdate _skeletalmesh (Variables|Default|GetMeshSkeletal) true)
        (Utilities|FlowControl|Delay 0.025)
        (Physics|SetSimulatePhysics (Variables|Default|GetSkeletalMesh) true)))))

(event Custom|Randomize%20Selected
  ;[1 1 1] Editor Buttons and Generation
  (CallFunction|Generate))

(event Custom|OpenLuggage
  (bind _transform_original (Variables|Default|GetTransform_Original))
  (bind _dynamicmesh (Variables|Default|GetDynamicMesh))
  (if (Variables|Default|GetDynamicSkeletalSpawned)
    (if (Variables|Default|GetCanSimulatedMeshesBeLooted?)
      (bind _output_get (Variables|Default|SetOpen (not (Variables|Default|GetOpen)) :!label _label))
      (Audio|SpawnSoundAttached (select _output_get (Variables|Default|GetSoundOpen) (Variables|Default|GetSoundClosed)) (Variables|Default|GetDefaultSceneRoot) "None" "0, 0, 0" "0, 0, 0" "SnapToTarget" false 1.0 1.0 0.0 0 0)
      (Utilities|IsValid (Variables|Default|GetDynamicMesh)
        (:Is%20Valid
          (Effects|SpawnEmitterAttached (Variables|Default|GetParticle) (Variables|Default|GetDynamicMesh) "None" "0, 0, 0" "0, 0, 0" (.scale _transform_original) "SnapToTargetIncludingScale"))
        (:Is%20Not%20Valid
          (Effects|SpawnEmitterAttached (Variables|Default|GetParticle) (Variables|Default|GetBox) "None" "0, 0, 0" "0, 0, 0" (.scale _transform_original) "SnapToTargetIncludingScale")))
      (if (not (Variables|Default|GetDynamicSkeletalSpawned))
        (Components|StaticMesh|SetStaticMesh _dynamicmesh (select (Variables|Default|GetOpen) (Variables|Default|GetMeshOpened) (Variables|Default|GetMeshClosed)))
        (Rendering|Material|SetMaterial _dynamicmesh 0 (Variables|Default|GetAssignMaterial))
        (Transformation|SetRelativeTransform (Variables|Default|GetDynamicMesh) (Variables|Default|GetTransform_Original) false false)))
    (else
      (Utilities|DestroyInstance)
      (goto _label))))

(event Custom|Randomize%20All%20Similar
  ;[1 1 1] Editor Buttons and Generation
  (bind _outactors (Actor|GetAllActorsOfClass (Utilities|GetClass self)))
  (for _array_element _outactors
    (CallFunction|Generate _array_element)))

(event EventBeginPlay
  ;[1 1 1] Some variables need to be initialized or they will be forgotten when set by the randomize event in the editor
  (Variables|Default|SetTransform_Original (Transformation|GetRelativeTransform (Variables|Default|GetInstancedStaticMesh)))
  (bind _returnvalue (AddComponent|AddStaticMeshComponent false))
  (Variables|Default|SetDynamicMesh _returnvalue)
  (if (Variables|Default|GetIsOpen?)
    (Variables|Default|SetOpen true)
    (else
      (Variables|Default|SetOpen false))))

(fn ConstructionScript)

(fn OnOpen)

(fn PlayEffects)