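; BP_Spawner continuously spawns physics-simulated fabric suitcases around its own location, producing a stream of tumbling luggage.
; From BeginPlay, a self-looping retriggerable delay spawns a SkeletalMeshActor at short intervals, randomly offset in X and Y, and assigns it the suitcase mesh.
; Each suitcase receives a randomized impulse biased toward world +Y.
; The loop has no stop condition, spawn cap or cleanup.
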(event EventBeginPlay
  (bind _self self)
  (bind _returnvalue (Transformation|GetActorTransform _self))
  (Utilities|FlowControl|RetriggerableDelay 0.05 :!label _label)
  (bind _returnvalue_2 (Game|SpawnActorfromClass "/Script/Engine.SkeletalMeshActor" (Math|Transform|MakeTransform (Math|Vector|MakeVector (Math|Random|RandomFloatinRange (+ (.x (.location _returnvalue)) -1.5e+02) (+ (.x (.location _returnvalue)) 1.5e+02)) (Math|Random|RandomFloatinRange (+ (.y (.location _returnvalue)) -1.5e+02) (+ (.y (.location _returnvalue)) 1.5e+02)) (.z (.location _returnvalue))) (.rotation _returnvalue) "1.000000,1.000000,1.000000") "Undefined" "MultiplyWithRoot" 0 0))
  (Components|SkinnedMesh|SetSkinnedAssetandUpdate (Variables|/Script/Engine.SkeletalMeshActor|GetSkeletalMeshComponent _returnvalue_2) "/Game/YI_Luggage_A/Meshes/Luggage_A/Skeletal/SK_Suitcase_Fabric.SK_Suitcase_Fabric" true)
  (Physics|SetSimulatePhysics (Variables|/Script/Engine.SkeletalMeshActor|GetSkeletalMeshComponent _returnvalue_2) true)
  (Physics|AddImpulse (Variables|/Script/Engine.SkeletalMeshActor|GetSkeletalMeshComponent _returnvalue_2) (Math|Vector|MakeVector (Math|Random|RandomFloatinRange -5e+02 5e+02) (Math|Random|RandomFloatinRange 2.5e+02 7.5e+02) (Math|Random|RandomFloatinRange -5e+02 5e+02)) "None" false)
  (goto _label))

(event Collision|EventActorBeginOverlap
  (params (OtherActor :type Actor%20Object%20Reference)))

(event EventTick
  (params (DeltaSeconds :type Float%20%28single-precision%29)))

(fn ConstructionScript)